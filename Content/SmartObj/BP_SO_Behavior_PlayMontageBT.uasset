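; BP_SO_Behavior_PlayMontageBT is a Smart Object behavior that currently only checks and prints claim state for the triggering character.
; On trigger it stores the avatar, reads a claim handle from its Blackboard via KeyName, and tests validity.
; It prints the avatar's name or "no BB", then immediately ends the behavior.
; Despite the asset name, the T-pose montage playback node is disconnected and never runs.
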(event GameplayBehavior|EventOnTriggeredCharacter
  (params (Avatar :type Character%20Object%20Reference) (Config :type Gameplay%20Behavior%20Config%20Object%20Reference) (SmartObjectOwner :type Actor%20Object%20Reference))
  (bind _output_get (Variables|Default|SetAvatar Avatar))
  (bind _returnvalue (Class|SmartObjectBlueprintFunctionLibrary|GetValueasSOClaimHandle (AI|GetBlackboard Avatar) (Variables|Default|GetKeyName)))
  (bind _returnvalue_2 (Class|SmartObjectBlueprintFunctionLibrary|IsValidSmartObjectClaimHandle _returnvalue))
  (if _returnvalue_2
    (Development|PrintString Avatar (Utilities|GetDisplayName _output_get))
    (else
      (Development|PrintString 0 "no BB" true true "(R=0.000000,G=0.063842,B=1.000000,A=1.000000)")))
  (GameplayBehavior|EndBehavior (Variables|Default|GetAvatar)))